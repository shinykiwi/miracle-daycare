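; Base actor for inspectable objects such as BP_Item and BP_Letter, with rotation and task counting.
; Mouse wheel input yaws the actor in fixed steps, while StartInspect only prints debug text because its input handoff nodes are disconnected.
; SetTasks casts self to either child class and adjusts TasksTotal and TasksComplete from its clean or read state, using TasksSet and a DoOnce to separate setup from completion.
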(event Custom|Start%20Inspect
  (params (Inspector :type Actor%20Object%20Reference))
  (Development|PrintString "INSPECTING" true true "(R=0.000000,G=0.660000,B=1.000000,A=1.000000)" 1e+01))

(event Custom|SetTasks
  (bind _self self)
  (bind _asbp_item (Utilities|Casting|CastToBP_Item _self)
    (:then
      (if (Variables|/Game/Blueprints/BP_Item.BP_Item_C|GetisClean _asbp_item)
        (if (Variables|Default|GetTasksSet)
          (Variables|Default|SetTasksComplete (+ (Variables|Default|GetTasksComplete) 1))
          (if true :!label _label
            _
            (else
              (Variables|Default|SetTasksTotal (+ (Variables|Default|GetTasksTotal) 1))))
          (Utilities|FlowControl|DoOnce false :!label _label_2
            (:Completed
              (Variables|Default|SetTasksSet true))))
        (else
          (Variables|Default|SetTasksTotal (+ (Variables|Default|GetTasksTotal) 1))
          (goto _label))))
    (:CastFailed
      (bind _asbp_letter (Utilities|Casting|CastToBP_Letter _self)
        (:then
          (if (Variables|Default|GetTasksSet)
            (if (Variables|/Game/Blueprints/BP_Letter.BP_Letter_C|GetisRead _asbp_letter)
              (Variables|Default|SetTasksComplete (+ (Variables|Default|GetTasksComplete) 1)))
            (else
              (Variables|Default|SetTasksTotal (+ (Variables|Default|GetTasksTotal) 1))
              (goto _label_2))))
        (:CastFailed
          (Development|PrintString "YIKES UR CODE SUCKS"))))))

(event Input|MouseEvents|MouseWheelUp
  (params (Key :type Key%20Structure :default "None"))
  (bind _returnvalue (Transformation|GetActorRotation))
  (:Pressed
    (Transformation|SetActorRotation (Math|Rotator|MakeRotator (.roll _returnvalue) (.pitch _returnvalue) (+ (.yaw _returnvalue) 2e+01)))))

(event Input|MouseEvents|MouseWheelDown
  (params (Key :type Key%20Structure :default "None"))
  (bind _returnvalue (Transformation|GetActorRotation))
  (:Pressed
    (Transformation|SetActorRotation (Math|Rotator|MakeRotator (.roll _returnvalue) (.pitch _returnvalue) (- (.yaw _returnvalue) 2e+01)))))

(fn ConstructionScript)