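; BP_Letter is a readable letter actor that the player opens and closes with E when nearby.
; On BeginPlay it creates the W_Letter widget, adds it to the viewport and hides it.
; Overlapping its Sphere enables input on the actor and leaving disables it, so E works only in range.
; A FlipFlop on E alternates showing and hiding the widget, each with its own paper sound.
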(event OnComponentBeginOverlap(Sphere)
  (params (OverlappedComponent :type Primitive%20Component%20Object%20Reference) (OtherActor :type Actor%20Object%20Reference) (OtherComp :type Primitive%20Component%20Object%20Reference) (OtherBodyIndex :type Integer) (bFromSweep :type Boolean) (SweepResult :type Hit%20Result%20Structure%20%28by%20ref%29))
  ;[0 0.01254 0.04688] Only turn on input when the player is close enough to the object
  (Input|EnableInput (Game|GetPlayerController 0)))

(event OnComponentEndOverlap(Sphere)
  (params (OverlappedComponent :type Primitive%20Component%20Object%20Reference) (OtherActor :type Actor%20Object%20Reference) (OtherComp :type Primitive%20Component%20Object%20Reference) (OtherBodyIndex :type Integer))
  ;[0 0.01254 0.04688] Only turn on input when the player is close enough to the object
  (Input|DisableInput (Game|GetPlayerController 0)))

(event EventBeginPlay
  (bind _returnvalue (UserInterface|CreateWidget "/Game/HUDs/W_Letter.W_Letter_C"))
  (bind _output_get (Variables|Default|SetWidgetREF _returnvalue))
  (UserInterface|Viewport|AddtoViewport _output_get 0)
  (Widget|SetVisibility _output_get "Hidden"))

(event Collision|EventActorBeginOverlap
  (params (OtherActor :type Actor%20Object%20Reference)))

(event EventTick
  (params (DeltaSeconds :type Float%20%28single-precision%29)))

(event Input|KeyboardEvents|E
  (params (Key :type Key%20Structure :default "None"))
  (:Pressed
    (Utilities|FlowControl|FlipFlop
      (:A
        (Widget|SetVisibility (stale EventBeginPlay _output_get) "Visible")
        (Audio|PlaySound2D "/Game/HorrorEngine/Audio/Paper/Paper07.Paper07" 1.0 1.0 0.0 0 0))
      (:B
        (Widget|SetVisibility (stale EventBeginPlay _output_get) "Hidden")
        (Audio|PlaySound2D "/Game/HorrorEngine/Audio/Paper/Paper08.Paper08" 1.0 1.0 0.0 0 0)))))

(fn ConstructionScript)