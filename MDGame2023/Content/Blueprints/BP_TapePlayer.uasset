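; BP_TapePlayer is an interactable tape player that visually loads a tape once the BP_Tape reference reports HasTape.
; Interact passes a DoOnce, reveals the tape mesh, then runs the sash macro and a timeline that slides the tape inside.
; The sash macro rotates a SpringArm by timeline.
; Tick re-fetches the first BP_Tape every frame, while CasttoTV caches the first BP_TV, unused here.
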(event Custom|Interact
  (if (Variables|/Game/Blueprints/BP_Tape.BP_Tape_C|GetHas%20Tape (Variables|Default|GetTape%20REF))
    (Utilities|FlowControl|DoOnce false
      (:Completed
        (Rendering|SetVisibility (Variables|Default|GetTape) true false)
        (|Open/CloseSash
          (:get%20tape%20in
            (bind _tape_inside (Timeline|Tape%20in Play)
              (:Update
                (Transformation|SetRelativeLocation (Variables|Default|GetTape) (Math|Vector|Lerp(Vector) (Variables|Default|GetTape%20Location%20A) (Variables|Default|GetTape%20Location%20B) _tape_inside) false false)))))))))

(event Custom|Cast%20to%20TV
  (bind _outactors (Actor|GetAllActorsOfClass "/Game/Blueprints/BP_TV.BP_TV_C"))
  (Variables|Default|SetTV%20REF (Utilities|Array|Get(acopy) _outactors)))

(event EventBeginPlay)

(event Collision|EventActorBeginOverlap
  (params (OtherActor :type Actor%20Object%20Reference)))

(event EventTick
  (params (DeltaSeconds :type Float%20%28single-precision%29))
  (bind _outactors (Actor|GetAllActorsOfClass "/Game/Blueprints/BP_Tape.BP_Tape_C"))
  (Variables|Default|SetTape%20REF (Utilities|Array|Get(acopy) _outactors)))

(fn ConstructionScript)