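; Pickup item actor that the first-person character can carry, drop or place on a table.
; Sphere overlap gates its input: E attaches it to the character's hand socket and calls HasItem, or detaches it with physics simulation.
; While held, G snaps it to the SnapPoint of the character's referenced table when in range.
; ToggleDrop flip-flops whether dropping with E is allowed.
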(event OnComponentBeginOverlap(Sphere)
  (params (OverlappedComponent :type Primitive%20Component%20Object%20Reference) (OtherActor :type Actor%20Object%20Reference) (OtherComp :type Primitive%20Component%20Object%20Reference) (OtherBodyIndex :type Integer) (bFromSweep :type Boolean) (SweepResult :type Hit%20Result%20Structure%20%28by%20ref%29))
  ;[0 0.01254 0.04688] Only turn on input when the player is close enough to the object
  (Input|EnableInput (Game|GetPlayerController 0)))

(event OnComponentEndOverlap(Sphere)
  (params (OverlappedComponent :type Primitive%20Component%20Object%20Reference) (OtherActor :type Actor%20Object%20Reference) (OtherComp :type Primitive%20Component%20Object%20Reference) (OtherBodyIndex :type Integer))
  ;[0 0.01254 0.04688] Only turn on input when the player is close enough to the object
  (Input|DisableInput (Game|GetPlayerController 0)))

(event Custom|ToggleDrop
  (Utilities|FlowControl|FlipFlop
    (:A
      (Variables|Default|SetisDropDisabled true))
    (:B
      (Variables|Default|SetisDropDisabled false))))

(event Input|KeyboardEvents|E
  (params (Key :type Key%20Structure :default "None"))
  (bind _staticmesh (Variables|Default|GetStaticMesh))
  (:Pressed
    (if (Variables|Default|GetisPickedUp)
      (if (not (Variables|Default|GetisDropDisabled))
        ;[0 0.01785 0.0625] Dropping the item
        (Transformation|DetachFromActor "KeepWorld" "KeepWorld" "KeepWorld")
        (Collision|SetCollisionEnabled _staticmesh "PhysicsOnly")
        (Physics|SetSimulatePhysics _staticmesh true)
        (Variables|Default|SetisPickedUp false))
      (else
        ;[0 0.01785 0.0625] Picking up the item
        (bind _asbp_first_person_character (Utilities|Casting|CastToBP_FirstPersonCharacter (stale OnComponentBeginOverlap(Sphere) OtherActor)))
        (bind _returnvalue (Transformation|AttachComponentToComponent (Variables|/Game/FirstPerson/Blueprints/BP_FirstPersonCharacter.BP_FirstPersonCharacter_C|GetFirstPersonMesh _asbp_first_person_character) "hand_rSocket" "SnapToTarget" "SnapToTarget" "SnapToTarget" true))
        (Variables|Default|SetisPickedUp _returnvalue)
        (Default|HasItem _asbp_first_person_character)))))

(event Input|KeyboardEvents|G
  (params (Key :type Key%20Structure :default "None"))
  (bind _returnvalue (Actor|GetAttachParentActor))
  (:Pressed
    (if (Variables|Default|GetisPickedUp)
      (bind _asbp_first_person_character (Utilities|Casting|CastToBP_FirstPersonCharacter _returnvalue)
        (:then
          (if (Variables|/Game/FirstPerson/Blueprints/BP_FirstPersonCharacter.BP_FirstPersonCharacter_C|GetInTableRange _asbp_first_person_character)
            (if (Utilities|IsValid (Variables|/Game/FirstPerson/Blueprints/BP_FirstPersonCharacter.BP_FirstPersonCharacter_C|GetTableREF _asbp_first_person_character))
              (Transformation|DetachFromActor "KeepWorld" "KeepWorld" "KeepWorld")
              (Transformation|AttachActorToActor (Variables|/Game/FirstPerson/Blueprints/BP_FirstPersonCharacter.BP_FirstPersonCharacter_C|GetTableREF _asbp_first_person_character) "SnapPoint" "SnapToTarget" "SnapToTarget" "SnapToTarget" true))))
        (:CastFailed
          (Development|PrintString (Utilities|GetDisplayName _returnvalue) true true "(R=0.000000,G=0.660000,B=1.000000,A=1.000000)" 1e+01))))))

(fn ConstructionScript)