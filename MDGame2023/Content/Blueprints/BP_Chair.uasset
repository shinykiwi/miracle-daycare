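; BP_Chair is the seat at the inspection table where the player sorts through items.
; Sphere overlap enables input; right-click blends to the inspect camera and opens W_Inspect, and Left Shift exits.
; Next banks a finished item in GI_Main's inventory and snaps a random "ItemsToSort" inspectable onto the table.
; Read, Clean and Combine act on letters or items, with Read and Clean refreshing the task counter that unlocks Next.
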(event OnComponentBeginOverlap(Sphere)
  (params (OverlappedComponent :type Primitive%20Component%20Object%20Reference) (OtherActor :type Actor%20Object%20Reference) (OtherComp :type Primitive%20Component%20Object%20Reference) (OtherBodyIndex :type Integer) (bFromSweep :type Boolean) (SweepResult :type Hit%20Result%20Structure%20%28by%20ref%29))
  ;[0 0.01254 0.04688] Only turn on input when the player is close enough to the object
  (Input|EnableInput (Game|GetPlayerController 0))
  (bind _output_get (Variables|Default|SetCharacterREF OtherActor)))

(event OnComponentEndOverlap(Sphere)
  (params (OverlappedComponent :type Primitive%20Component%20Object%20Reference) (OtherActor :type Actor%20Object%20Reference) (OtherComp :type Primitive%20Component%20Object%20Reference) (OtherBodyIndex :type Integer))
  ;[0 0.01254 0.04688] Only turn on input when the player is close enough to the object
  (Input|DisableInput (Game|GetPlayerController 0)))

(event Custom|OnReadButton_Clicked
  ;[0 0.01785 0.0625] Read
  (Development|PrintString "READING")
  (bind _asbp_letter (Utilities|Casting|CastToBP_Letter (Variables|Default|GetCurrentItem)))
  (Default|Read _asbp_letter)
  (Utilities|FlowControl|Sequence
    (:then_0
      (bind _astext (Utilities|Casting|CastToTextBlock (Class|PanelWidget|GetChildat (Variables|/Game/HUDs/W_Inspect.W_Inspect_C|GetReadButton (Variables|Default|GetHUDREF)))))
      (if true
        (Utilities|FlowControl|FlipFlop
          (:A
            (Variables|/Script/UMG.TextBlock|SetText _astext "Close"))
          (:B
            (Variables|/Script/UMG.TextBlock|SetText _astext "Read")))))
    (:then_1
      (Utilities|FlowControl|DoOnce false
        (:Completed
          (CallFunction|UpdatedStatus))))))

(event Custom|OnNextButton_Clicked
  (bind _hudref (Variables|Default|GetHUDREF))
  ;[0 0.01785 0.0625] Next button behaviour
  (if (Utilities|IsValid (Variables|Default|GetCurrentItem))
    (if (== (Variables|/Game/Blueprints/BP_Inspectable.BP_Inspectable_C|GetTasksComplete (Variables|Default|GetCurrentItem)) (Variables|/Game/Blueprints/BP_Inspectable.BP_Inspectable_C|GetTasksTotal (Variables|Default|GetCurrentItem)))
      (Class|Border|SetBrushColor (Variables|/Game/HUDs/W_Inspect.W_Inspect_C|GetStatus (Variables|Default|GetHUDREF)) "(R=0.410753,G=0.461544,B=0.588542,A=1.000000)")
      (Transformation|DetachFromActor (Variables|Default|GetCurrentItem) "KeepRelative" "KeepRelative" "KeepRelative")
      (bind _asgi_main (Utilities|Casting|CastToGI_Main (Game|GetGameInstance)))
      (Utilities|Array|Add (Variables|/Game/AN-IMPORTANT-FOLDER/GI_Main.GI_Main_C|GetInventoryItems _asgi_main) (Variables|Default|GetCurrentItem))
      (Transformation|SetActorLocation (Variables|Default|GetCurrentItem) "0, 0, 0" false true)
      (Variables|/Script/Engine.Actor|SetTags (Variables|Default|GetCurrentItem) (Utilities|Array|MakeArray "None"))
      (bind _outactors (Actor|GetAllActorsOfClasswithTag "/Game/Blueprints/BP_Inspectable.BP_Inspectable_C" "ItemsToSort" :!label _label))
      (bind _output_get (Variables|Default|SetCurrentItem (.OutItem (Utilities|Array|Random _outactors))))
      (bind _returnvalue (Transformation|AttachComponentToComponent _output_get (Variables|Default|GetDiningTable_b) "SnapPoint" "SnapToTarget" "SnapToTarget" "SnapToTarget" true))
      (if _returnvalue
        (Default|StartInspect _output_get (Variables|Default|GetCharacterREF))
        (Variables|Default|SetisInspecting true)
        (Utilities|FlowControl|Sequence
          (:then_0
            ;[0 0.01785 0.0625] Updating the item description on-screen
            (Variables|/Script/UMG.TextBlock|SetText (Variables|/Game/HUDs/W_Inspect.W_Inspect_C|GetItemName _hudref) (Variables|/Game/Blueprints/BP_Inspectable.BP_Inspectable_C|GetItemName (Variables|Default|GetCurrentItem)))
            (Variables|/Script/UMG.TextBlock|SetText (Variables|/Game/HUDs/W_Inspect.W_Inspect_C|GetItemDescription _hudref) (Variables|/Game/Blueprints/BP_Inspectable.BP_Inspectable_C|GetItemDescription (Variables|Default|GetCurrentItem))))
          (:then_1
            (CallFunction|ToggleNextButton false))
          (:then_2
            (CallFunction|UpdatedStatus))))
      (else
        (Development|PrintString "ERROR! TASKS ARENT DONE" true true "(R=1.000000,G=0.000000,B=0.030794,A=1.000000)")))
    (else
      (goto _label))))

(event Custom|OnCleanButton_Clicked
  ;[0 0.01785 0.0625] Clean
  (Development|PrintString "CLEANING")
  (bind _asbp_item (Utilities|Casting|CastToBP_Item (Variables|Default|GetCurrentItem)))
  (if (Variables|/Game/Blueprints/BP_Item.BP_Item_C|GetisClean _asbp_item)
    (Development|PrintString "This object is already clean!")
    (else
      (Default|Clean _asbp_item)
      (CallFunction|UpdatedStatus))))

(event Custom|UpdatedStatus
  (bind _currentitem (Variables|Default|GetCurrentItem))
  (bind _hudref (Variables|Default|GetHUDREF))
  (bind _taskscomplete (Variables|/Game/Blueprints/BP_Inspectable.BP_Inspectable_C|GetTasksComplete _currentitem))
  (bind _status (Variables|/Game/HUDs/W_Inspect.W_Inspect_C|GetStatus _hudref))
  (bind _taskstotal (Variables|/Game/Blueprints/BP_Inspectable.BP_Inspectable_C|GetTasksTotal _currentitem))
  (Default|SetTasks (Variables|Default|GetCurrentItem))
  (bind _astext (Utilities|Casting|CastToTextBlock (Class|PanelWidget|GetChildat _status)))
  (Variables|/Script/UMG.TextBlock|SetText _astext (Utilities|Text|ToText(String) (Utilities|String|Append (Utilities|String|Append (Utilities|String|MakeLiteralString (Utilities|String|ToString(Byte) _taskscomplete)) (Utilities|String|MakeLiteralString " / ")) (Utilities|String|MakeLiteralString (Utilities|String|ToString(Byte) _taskstotal)))))
  (if (== _taskscomplete _taskstotal)
    (Class|Border|SetBrushColor _status "(R=0.128384,G=0.708333,B=0.193378,A=1.000000)")
    (CallFunction|ToggleNextButton true)))

(event Custom|ToggleNextButton
  (params (IsEnabled :type Boolean))
  ;[0 0.01785 0.0625] Next button behaviour
  (Variables|/Script/UMG.Widget|SetbIsEnabled (Variables|/Game/HUDs/W_Inspect.W_Inspect_C|GetNextButton (Variables|Default|GetHUDREF)) IsEnabled))

(event Custom|OnCombineButton_Clicked
  (bind _currentitem (Variables|Default|GetCurrentItem))
  (if (Utilities|IsValid _currentitem)
    (bind _asbp_item (Utilities|Casting|CastToBP_Item _currentitem))
    (Development|PrintString "GOT TO COMBINE")
    (Default|Combine _asbp_item)))

(event Input|MouseEvents|RightMouseButton
  (params (Key :type Key%20Structure :default "None"))
  (bind _returnvalue (Game|GetPlayerController 0))
  (bind _currentitem (Variables|Default|GetCurrentItem))
  ;[0 0.01785 0.0625] Sitting Down
  (:Pressed
    (if (not (Variables|Default|GetisSitting))
      (bind _returnvalue_2 (Actor|GetActorOfClass "/Game/Blueprints/BP_InspectCamera.BP_InspectCamera_C"))
      (Game|Player|SetViewTargetwithBlend _returnvalue _returnvalue_2 1.0 "VTBlend_EaseIn" 0.5 false)
      (Audio|PlaySoundatLocation "/Game/HorrorEngine/Audio/DoorsAndFurnitures/DrawerOpen01.DrawerOpen01" (Transformation|GetActorLocation) "0, 0, 0" 1.0 1.0 0.0 0 0 0 0)
      (Variables|Default|SetisSitting true)
      ;[0 0.01785 0.0625] Creating the inspect HUD
      (bind _returnvalue_3 (UserInterface|CreateWidget "/Game/HUDs/W_Inspect.W_Inspect_C"))
      (bind _output_get (Variables|Default|SetHUDREF _returnvalue_3))
      (UserInterface|Viewport|AddtoViewport _output_get 0)
      (Variables|/Script/Engine.PlayerController|SetbShowMouseCursor _returnvalue true)
      (Utilities|FlowControl|Sequence
        (:then_0
          ;[0 0.01785 0.0625] Next button behaviour
          (EventDispatchers|AssignOnClicked (Variables|/Game/HUDs/W_Inspect.W_Inspect_C|GetNextButton (Variables|Default|GetHUDREF)) (delegate Custom|OnNextButton_Clicked)))
        (:then_1
          ;[0 0.01785 0.0625] Read
          (EventDispatchers|BindEventtoOnClicked (Variables|/Game/HUDs/W_Inspect.W_Inspect_C|GetReadButton (Variables|Default|GetHUDREF)) (delegate Custom|OnReadButton_Clicked)))
        (:then_2
          ;[0 0.01785 0.0625] Clean
          (EventDispatchers|BindEventtoOnClicked (Variables|/Game/HUDs/W_Inspect.W_Inspect_C|GetCleanButton (Variables|Default|GetHUDREF)) (delegate Custom|OnCleanButton_Clicked)))
        (:then_3
          (EventDispatchers|BindEventtoOnClicked (Variables|/Game/HUDs/W_Inspect.W_Inspect_C|GetCombineButton (Variables|Default|GetHUDREF)) (delegate Custom|OnCombineButton_Clicked))
          (if (Utilities|IsValid _currentitem)
            (Utilities|Casting|CastToBP_Item _currentitem
              (:CastFailed
                (Widget|SetIsEnabled (Variables|/Game/HUDs/W_Inspect.W_Inspect_C|GetCombineButton (Variables|Default|GetHUDREF)) false)))))))))

(event Input|KeyboardEvents|LeftShift
  (params (Key :type Key%20Structure :default "None"))
  (bind _returnvalue (Game|GetPlayerController 0))
  ;[0.1562 0.0236 0.0236] Exiting the inspect table
  (:Pressed
    (if (Variables|Default|GetisSitting)
      (Game|Player|SetViewTargetwithBlend _returnvalue (stale OnComponentBeginOverlap(Sphere) _output_get) 1.0 "VTBlend_Linear" 0.5 false)
      (Widget|SetVisibility (Variables|Default|GetHUDREF) "Hidden") ; Hides the HUD
      (Variables|/Script/Engine.PlayerController|SetbShowMouseCursor _returnvalue false) ; Hides the mouse cursor
      (Variables|Default|SetisSitting false) ; The player is no longer sitting
      (Input|DisableInput (Variables|Default|GetCurrentItem) _returnvalue) ; Takes the input away from the item
      (Input|EnableInput (Variables|Default|GetCharacterREF) _returnvalue) ; Gives the input back to the player
    )))

(fn ConstructionScript)