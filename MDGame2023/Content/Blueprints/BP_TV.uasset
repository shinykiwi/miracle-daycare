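; BP_TV is a television actor that plays a VHS video on its screen when ShowVideoOnTv is called.
; After a one-second delay it opens a media source, routes audio through a MediaSound component and swaps the screen's material slot to the video material.
; When playback reaches its end, it switches the screen to a noise material and notifies the first BP_TapePlayer found in the level that the tape ended.
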(event Custom|Show%20Video%20On%20Tv
  (bind _media_player (Variables|Default|GetMedia%20Player))
  (Utilities|FlowControl|Delay 1.0)
  (Media|MediaPlayer|OpenSource _media_player (Variables|Default|GetMedia%20Source))
  (Media|MediaSoundComponent|SetMediaPlayer (Variables|Default|GetMediaSound) _media_player)
  (Rendering|Material|SetMaterial (Variables|Default|GetStaticMesh) 1 "/Game/Videos/vhsbaldi_Inst.vhsbaldi_Inst")
  (Media|MediaPlayer|BindEventtoOnEndReached _media_player (delegate Custom|VHS%20Tape%20ending)))

(event Custom|VHS%20Tape%20ending
  (Rendering|Material|SetMaterial (Variables|Default|GetStaticMesh) 1 "/Game/HorrorEngine/Materials/He_Noise2.He_Noise2")
  (bind _outactors (Actor|GetAllActorsOfClass "/Game/Blueprints/BP_TapePlayer.BP_TapePlayer_C"))
  (Default|IfTapeHadEnded (Utilities|Array|Get(acopy) _outactors)))

(event EventBeginPlay)

(event Collision|EventActorBeginOverlap
  (params (OtherActor :type Actor%20Object%20Reference)))

(event EventTick
  (params (DeltaSeconds :type Float%20%28single-precision%29)))

(fn ConstructionScript)