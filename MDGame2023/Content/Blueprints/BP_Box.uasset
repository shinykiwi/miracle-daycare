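; BP_Box is an interactable fish crate that the player opens and closes with E to show or hide an item widget.
; A box overlap enables input on entry and disables it on exit.
; BeginPlay creates a hidden W_Items widget and populates it, and each toggle swaps the crate mesh and widget visibility.
; A pop sound and a GI_Main cast are present but unconnected.
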(event OnComponentBeginOverlap(Box)
  (params (OverlappedComponent :type Primitive%20Component%20Object%20Reference) (OtherActor :type Actor%20Object%20Reference) (OtherComp :type Primitive%20Component%20Object%20Reference) (OtherBodyIndex :type Integer) (bFromSweep :type Boolean) (SweepResult :type Hit%20Result%20Structure%20%28by%20ref%29))
  ;[0 0.01785 0.0625] Enable/disable input based on overlap
  (Input|EnableInput (Game|GetPlayerController 0)))

(event OnComponentEndOverlap(Box)
  (params (OverlappedComponent :type Primitive%20Component%20Object%20Reference) (OtherActor :type Actor%20Object%20Reference) (OtherComp :type Primitive%20Component%20Object%20Reference) (OtherBodyIndex :type Integer))
  ;[0 0.01785 0.0625] Enable/disable input based on overlap
  (Input|DisableInput (Game|GetPlayerController 0)))

(event EventBeginPlay
  (bind _returnvalue (UserInterface|CreateWidget "/Game/HUDs/W_Items.W_Items_C"))
  (bind _output_get (Variables|Default|SetHUDREF _returnvalue))
  (Default|PopulateItems _output_get)
  (UserInterface|Viewport|AddtoViewport _output_get 0)
  (Widget|SetVisibility _output_get "Hidden"))

(event Input|KeyboardEvents|E
  (params (Key :type Key%20Structure))
  (bind _staticmesh (Variables|Default|GetStaticMesh))
  ;[0 0.01785 0.0625] Opening the box
  (:Pressed
    (if (Variables|Default|GetisOpen)
      (Components|StaticMesh|SetStaticMesh _staticmesh "/Game/EF_MollyGreg/Meshes/FishCrate_c_Closed.FishCrate_c_Closed")
      (Variables|Default|SetisOpen false)
      (Widget|SetVisibility (Variables|Default|GetHUDREF) "Hidden")
      (else
        (bind _returnvalue (Components|StaticMesh|SetStaticMesh _staticmesh "/Game/EF_MollyGreg/Meshes/FishCrate_c.FishCrate_c"))
        (Variables|Default|SetisOpen _returnvalue)
        (Widget|SetVisibility (Variables|Default|GetHUDREF) "Visible")))))

(fn ConstructionScript)